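; OrbActor_BP is a mini-game orb with a spinning swirl and two rings.
; Tick spins each mesh on its own axis, with ring speeds scaled by multipliers that are eased back from high or negative values.
; The easing is one branch chain, so the vertical multiplier only recovers while the horizontal one is in range.
; On destruction it blends the camera back to the player, restores walking, adds health and clears the mini-game flag.
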(event EventBeginPlay
  (Variables|Default|Sethorizontal_orb_ring (Variables|Default|GetOrb_ring_horizontal))
  (Variables|Default|Setvertical_orb_ring (Variables|Default|GetOrb_ring_vertical))
  (Variables|Default|Setswirl_orb (Variables|Default|GetOrb_swirl))
  (Variables|Default|SetRotationSpeedMultiplier_H 1.0)
  (Variables|Default|SetRotationSpeedMultiplier_V 1.0))

(event EventTick
  (params (DeltaSeconds :type Float%20%28single-precision%29))
  ;[1 1 1] Add natural spin to the meshes
  (Transformation|AddLocalRotation (Variables|Default|GetOrb_swirl) (Math|Rotator|MakeRotator 0.0 0.0 (* DeltaSeconds 5e+01)) false false)
  (Transformation|AddLocalRotation (Variables|Default|GetOrb_ring_vertical) (Math|Rotator|MakeRotator (* DeltaSeconds (* 12.0 (Variables|Default|GetRotationSpeedMultiplier_V))) 0.0 0.0) false false)
  (Transformation|AddLocalRotation (Variables|Default|GetOrb_ring_horizontal) (Math|Rotator|MakeRotator 0.0 (* DeltaSeconds (* 8.0 (Variables|Default|GetRotationSpeedMultiplier_H))) 0.0) false false)
  ;[1 1 1] Slow Down the multiplier speed after its been applied
  (if (> (Variables|Default|GetRotationSpeedMultiplier_H) 8.0)
    (Variables|Default|SetRotationSpeedMultiplier_H (- (Variables|Default|GetRotationSpeedMultiplier_H) (* (Utilities|Time|GetWorldDeltaSeconds) 25.0)))
    (elif (< (Variables|Default|GetRotationSpeedMultiplier_H) 0.0)
      (Variables|Default|SetRotationSpeedMultiplier_H (+ (Variables|Default|GetRotationSpeedMultiplier_H) (* (Utilities|Time|GetWorldDeltaSeconds) 25.0)))
      (elif (> (Variables|Default|GetRotationSpeedMultiplier_V) 12.0)
        (Variables|Default|SetRotationSpeedMultiplier_V (- (Variables|Default|GetRotationSpeedMultiplier_V) (* (Utilities|Time|GetWorldDeltaSeconds) 25.0)))
        (elif (< (Variables|Default|GetRotationSpeedMultiplier_V) 0.0)
          (Variables|Default|SetRotationSpeedMultiplier_V (+ (Variables|Default|GetRotationSpeedMultiplier_V) (* (Utilities|Time|GetWorldDeltaSeconds) 25.0))))))))

(event EventDestroyed
  (bind _player (Variables|Default|GetPlayer))
  (Development|PrintString "Orb Destroyed")
  (Game|Player|SetViewTargetwithBlend (Game|GetPlayerController 0) (Variables|Default|GetPlayer) 2.0 "VTBlend_Linear" 0.0 false)
  ;[1 1 1] Enable Movement
  (Pawn|Components|CharacterMovement|SetMovementMode (Variables|/Script/Engine.Character|GetCharacterMovement (Variables|Default|GetPlayer)) "MOVE_Walking" 0)
  (Class|UnnaturalGuardianCharacter|AddPlayerHealth _player (Variables|Default|GetPlayerHealthRecovery))
  (Variables|/Game/ThirdPersonCPP/Blueprints/BP_UnnaturalGuardianCharacter.BP_UnnaturalGuardianCharacter_C|SetPlayingMiniGame _player false))

(fn ConstructionScript)