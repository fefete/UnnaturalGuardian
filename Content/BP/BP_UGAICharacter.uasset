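; AI character that tracks whether it can see the Unnatural Guardian player and turns to face them.
; Each Tick, if the Blackboard Target is that character, it box-traces toward player 0's pawn over a RaycastMultiplier distance, drawing debug each frame.
; A hit on the player sets CanSeePlayer and snaps rotation toward Target; otherwise it clears the flag and Target.
; Target is only read or cleared here, never assigned.
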(event EventBeginPlay)

(event Collision|EventActorBeginOverlap
  (params (OtherActor :type Actor%20Object%20Reference)))

(event EventTick
  (params (DeltaSeconds :type Float%20%28single-precision%29))
  (bind _found (CallFunction|IsPlayerinSight))
  (if _found
    (Class|UGAICharacter|SetCanSeePlayer true)
    (CallFunction|RotatetoPlayer)
    (else
      (Class|UGAICharacter|SetCanSeePlayer false)
      (bind _returnvalue (AI|GetAIController self))
      (AI|Components|Blackboard|ClearValue (AI|GetBlackboard _returnvalue) (Utilities|Name|MakeLiteralName "Target")))))

(fn ConstructionScript)

(fn IsPlayerinSight
  (bind _returnvalue (Transformation|GetActorLocation))
  (bind _returnvalue_2 (AI|GetAIController self))
  (Utilities|Casting|CastToBP_UnnaturalGuardianCharacter (AI|Components|Blackboard|GetValueasObject (AI|GetBlackboard _returnvalue_2) (Utilities|Name|MakeLiteralName "Target"))
    (:then
      (bind (_outhit _returnvalue_3) (Class|KismetSystemLibrary|BoxTraceSingleforObjects _returnvalue (+ _returnvalue (* (Math|Vector|Normalize (- (Transformation|GetActorLocation (Pawn|GetControlledPawn (Game|GetPlayerController 0))) _returnvalue)) (Variables|Default|GetRaycastMultiplier))) "10.000000,10.000000,10.000000" "0, 0, 0" (Utilities|Array|MakeArray "ObjectTypeQuery3" "ObjectTypeQuery1" "ObjectTypeQuery4" "ObjectTypeQuery2") false 0 "ForOneFrame" true))
      (if _returnvalue_3
        (Utilities|Casting|CastToBP_UnnaturalGuardianCharacter (.HitActor (Collision|BreakHitResult _outhit))
          (:then
            (return true))
          (:CastFailed
            _)))
      (return false))
    (:CastFailed
      (return false))))

(fn RotatetoPlayer
  (bind _returnvalue (AI|GetAIController self))
  (bind _asbp_unnatural_guardian_character (Utilities|Casting|CastToBP_UnnaturalGuardianCharacter (AI|Components|Blackboard|GetValueasObject (AI|GetBlackboard _returnvalue) (Utilities|Name|MakeLiteralName "Target"))))
  (Transformation|SetActorRotation (Math|Rotator|FindLookatRotation (Transformation|GetActorLocation) (Transformation|GetActorLocation _asbp_unnatural_guardian_character))))