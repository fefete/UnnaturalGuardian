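; BP_LakeDamage is a hazard volume, a lake by its name, that drains the player's health while they are inside it.
; Box begin overlap with a BP_UnnaturalGuardianCharacter stores the player and enables damage, and the actor's end overlap disables it.
; While enabled, Tick subtracts a fixed per-second rate, scaled by delta time, directly from PlayerCurrentHealth without clamping, and prints the value for debugging.
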(event OnComponentBeginOverlap(Box)
  (params (OverlappedComponent :type Primitive%20Component%20Object%20Reference) (OtherActor :type Actor%20Object%20Reference) (OtherComp :type Primitive%20Component%20Object%20Reference) (OtherBodyIndex :type Integer) (bFromSweep :type Boolean) (SweepResult :type Hit%20Result%20Structure%20%28by%20ref%29))
  (bind _asbp_unnatural_guardian_character (Utilities|Casting|CastToBP_UnnaturalGuardianCharacter OtherActor))
  (Variables|Default|Setplayer _asbp_unnatural_guardian_character)
  (Variables|Default|SetDealDMG true))

(event EventBeginPlay)

(event Collision|EventActorBeginOverlap
  (params (OtherActor :type Actor%20Object%20Reference)))

(event EventTick
  (params (DeltaSeconds :type Float%20%28single-precision%29))
  (Variables|Default|SetDelta DeltaSeconds)
  (if (Variables|Default|GetDealDMG)
    (Development|PrintString (Utilities|String|ToString(Float) (- (Variables|/Script/UnnaturalGuardian.UnnaturalGuardianCharacter|GetplayerCurrentHealth_ (Variables|Default|Getplayer)) (* (Variables|Default|GetDelta) 65.0))) true true "(R=0.000000,G=0.660000,B=1.000000,A=1.000000)" 0.0)
    (Variables|/Script/UnnaturalGuardian.UnnaturalGuardianCharacter|SetplayerCurrentHealth_ (Variables|Default|Getplayer) (- (Variables|/Script/UnnaturalGuardian.UnnaturalGuardianCharacter|GetplayerCurrentHealth_ (Variables|Default|Getplayer)) (* (Variables|Default|GetDelta) 65.0)))))

(event Collision|EventActorEndOverlap
  (params (OtherActor :type Actor%20Object%20Reference))
  (bind _asbp_unnatural_guardian_character (Utilities|Casting|CastToBP_UnnaturalGuardianCharacter OtherActor))
  (Variables|Default|Setplayer _asbp_unnatural_guardian_character)
  (Variables|Default|SetDealDMG false))

(fn ConstructionScript)