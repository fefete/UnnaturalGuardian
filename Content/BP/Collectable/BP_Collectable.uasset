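; BP_Collectable is a collectable actor that shows either a 3D object or a 2D lore image.
; BeginPlay adds its own BP_UI widget to the viewport.
; ShowViewableAsset either swaps in MeshToSpawn, applying the camera's world transform offset in Y as a half-scale relative transform and printing it, or reveals the lore image.
; GetCollected destroys the actor, first hiding the image in 2D mode.
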(event EventBeginPlay
  (bind _returnvalue (UserInterface|CreateWidget "/Game/UI/BP_UI.BP_UI_C"))
  (bind _output_get (Variables|Default|SetUI _returnvalue))
  (UserInterface|Viewport|AddtoViewport _output_get 0))

(event Collision|EventActorBeginOverlap
  (params (OtherActor :type Actor%20Object%20Reference)))

(event EventTick
  (params (DeltaSeconds :type Float%20%28single-precision%29)))

(fn ConstructionScript)

(fn GetCollected
  (if (Variables|Default|GetShow3DObject)
    (Actor|DestroyActor)
    (elif (Variables|Default|GetShow2DImage)
      (Variables|/Game/UI/BP_UI.BP_UI_C|SetUI_LoreImage (Variables|Default|GetUI) "Hidden")
      (Actor|DestroyActor))))

(fn ShowViewableAsset
  (bind _playerviewcamera (Variables|Default|GetPlayerViewCamera))
  (bind _cameracomponent (Variables|/Script/Engine.CameraActor|GetCameraComponent _playerviewcamera))
  (bind _returnvalue (Transformation|GetWorldTransform _cameracomponent))
  (bind (_location _rotation) (Math|Transform|BreakTransform _returnvalue))
  (bind (_x _y _z) (Math|Vector|BreakVector _location))
  (bind _returnvalue_2 (- _y 1.5e+02))
  (bind _returnvalue_3 (Math|Vector|MakeVector _x _returnvalue_2 _z))
  (bind _returnvalue_4 (Math|Transform|MakeTransform _returnvalue_3 _rotation "0.500000,0.500000,0.500000"))
  (if (Variables|Default|GetShow3DObject)
    (Transformation|SetRelativeTransform (Variables|Default|GetcollectableMesh_) _returnvalue_4 false false)
    (Components|StaticMesh|SetStaticMesh (Variables|Default|GetcollectableMesh_) (Variables|Default|GetMeshToSpawn))
    (Development|PrintString (Utilities|String|ToString(Transform) _returnvalue_4))
    (elif (Variables|Default|GetShow2DImage)
      (Variables|/Game/UI/BP_UI.BP_UI_C|SetUI_LoreImage (Variables|Default|GetUI) "Visible"))))