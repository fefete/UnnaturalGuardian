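; End-screen game mode that respawns the player's Unnatural Guardian character after it is destroyed.
; BeginPlay caches the player character and binds its OnDestroyed event.
; After a short delay, the handler loads the save and spawns and possesses a new character at the saved checkpoint, or at SpawnLocation if SaveLevel is set or no save exists.
; Each respawn then calls the respawn event to rebind.
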(event Custom|PlayerDestroyed
  (params (DestroyedActor :type Actor%20Object%20Reference))
  (bind _returnvalue (Game|GetPlayerController 0))
  (Utilities|FlowControl|Delay 2.0)
  (bind _returnvalue_2 (SaveGame|DoesSaveGameExist "Save_001"))
  (if _returnvalue_2
    (bind _returnvalue_3 (SaveGame|LoadGamefromSlot "Save_001"))
    (bind _asgame_save (Utilities|Casting|CastToGameSave _returnvalue_3))
    (if (Variables|/Game/BP/Checkpoint/GameSave.GameSave_C|GetSaveLevel _asgame_save)
      (bind _returnvalue_4 (Game|SpawnActorfromClass "/Game/ThirdPersonCPP/Blueprints/BP_UnnaturalGuardianCharacter.BP_UnnaturalGuardianCharacter_C" (Variables|Default|GetSpawnLocation) "Undefined" 0 0))
      (Pawn|Possess _returnvalue _returnvalue_4)
      (CallFunction|RespawnEvent)
      (else
        (bind _returnvalue_5 (Game|SpawnActorfromClass "/Game/ThirdPersonCPP/Blueprints/BP_UnnaturalGuardianCharacter.BP_UnnaturalGuardianCharacter_C" (Math|Transform|MakeTransform (Variables|/Game/BP/Checkpoint/GameSave.GameSave_C|GetCheckpoint _asgame_save) "0, 0, 0" "0.600000,0.600000,0.600000") "Undefined" 0 0))
        (Pawn|Possess _returnvalue _returnvalue_5)
        (CallFunction|RespawnEvent)))
    (else
      (bind _returnvalue_6 (Game|SpawnActorfromClass "/Game/ThirdPersonCPP/Blueprints/BP_UnnaturalGuardianCharacter.BP_UnnaturalGuardianCharacter_C" (Variables|Default|GetSpawnLocation) "Undefined" 0 0))
      (Pawn|Possess (Game|GetPlayerController 0) _returnvalue_6)
      (CallFunction|RespawnEvent))))

(event Custom|Respawn_Event
  (bind _asunnatural_guardian_character (Utilities|Casting|CastToUnnaturalGuardianCharacter (Game|GetPlayerCharacter 0)))
  (bind _output_get (Variables|Default|SetCharacter _asunnatural_guardian_character))
  (Game|BindEventtoOnDestroyed _asunnatural_guardian_character (delegate Custom|PlayerDestroyed)))

(event EventBeginPlay
  (bind _asunnatural_guardian_character (Utilities|Casting|CastToUnnaturalGuardianCharacter (Game|GetPlayerCharacter 0)))
  (bind _output_get (Variables|Default|SetCharacter _asunnatural_guardian_character))
  (Game|BindEventtoOnDestroyed _asunnatural_guardian_character (delegate Custom|PlayerDestroyed)))

(event EventTick
  (params (DeltaSeconds :type Float%20%28single-precision%29)))

(fn ConstructionScript)