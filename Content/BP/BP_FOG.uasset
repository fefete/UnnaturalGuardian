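; BP_FOG is a fog controller that smoothly transitions Exponential Height Fog to new settings at runtime.
; ChangeFogValues stores a target density, a target directional inscattering exponent and a blend speed.
; Every Tick lerps the current fog values toward those targets using DeltaSeconds times the speed, giving an eased approach rather than a fixed-duration blend.
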(event EventBeginPlay)

(event Collision|EventActorBeginOverlap
  (params (OtherActor :type Actor%20Object%20Reference)))

(event EventTick
  (params (DeltaSeconds :type Float%20%28single-precision%29))
  (bind _lerpspeed (Variables|Default|GetLERPSpeed))
  (bind _exponentialheightfog (Variables|Default|GetExponentialHeightFog))
  (bind _returnvalue (* DeltaSeconds _lerpspeed))
  ;[1 1 1] Set new values to the fog
  (Class|ExponentialHeightFogComponent|SetDirectionalInscatteringExponent (Variables|Default|GetExponentialHeightFog) (Math|Float|Lerp (Variables|/Script/Engine.ExponentialHeightFogComponent|GetDirectionalInscatteringExponent _exponentialheightfog) (Variables|Default|GetChangeInscatteringTo) _returnvalue))
  (Class|ExponentialHeightFogComponent|SetFogDensity (Variables|Default|GetExponentialHeightFog) (Math|Float|Lerp (Variables|/Script/Engine.ExponentialHeightFogComponent|GetFogDensity _exponentialheightfog) (Variables|Default|GetChangeDensityTo) _returnvalue)))

(fn ConstructionScript)

(fn ChangeFogValues
  (params (Speed :type Float%20%28single-precision%29) (Density :type Float%20%28single-precision%29) (Inscattering :type Float%20%28single-precision%29))
  (Variables|Default|SetLERPSpeed Speed)
  (Variables|Default|SetChangeDensityTo Density)
  (Variables|Default|SetChangeInscatteringTo Inscattering))